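; BP_PlayerPawn is the player pawn, using the Gameplay Ability System and showing its attributes on the HUD.
; On BeginPlay it applies the GE_BasicRegen effect to itself for slow regeneration.
; Health, Mana and Strength change events cast the controller to BP_BasePlayerController and set the matching PrimaryUI glass ball to the current-to-max ratio.
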(event EventBeginPlay
  (|CallParentFunction)
  ;[1 1 1] 缓慢回复效果
  (GameplayEffects|ApplyGameplayEffectToSelf :self (Variables|Default|GetAbilitySystemComp) :GameplayEffectClass "/Game/Blueprints/Characters/Ability/GeneraGameplayEffect/GE_BasicRegen.GE_BasicRegen_C"))

(event Collision|EventActorBeginOverlap
  (params (OtherActor :type Actor%20Object%20Reference))
  (|CallParentFunction OtherActor) ; This node is disabled and will not be called.\nDrag off pins to build functionality.
)

(event EventTick
  (params (DeltaSeconds :type Float%20%28single-precision%29)))

(event EventOnHealthChange
  (params (Health :type Float%20%28single-precision%29) (MaxHealth :type Float%20%28single-precision%29))
  (bind _asbp_base_player_controller (Utilities|Casting|CastToBP_BasePlayerController (Pawn|GetController)))
  (Default|SetPercentage (Variables|/Game/UI/WBP_PrimaryUI.WBP_PrimaryUI_C|GetHealth_GlassBall (Variables|/Game/Blueprints/BP_BasePlayerController.BP_BasePlayerController_C|GetPrimaryUI _asbp_base_player_controller)) (/ Health MaxHealth)))

(event EventOnManaChange
  (params (Mana :type Float%20%28single-precision%29) (MaxMana :type Float%20%28single-precision%29))
  (bind _asbp_base_player_controller (Utilities|Casting|CastToBP_BasePlayerController (Pawn|GetController)))
  (Default|SetPercentage (Variables|/Game/UI/WBP_PrimaryUI.WBP_PrimaryUI_C|GetMana_GlassBall (Variables|/Game/Blueprints/BP_BasePlayerController.BP_BasePlayerController_C|GetPrimaryUI _asbp_base_player_controller)) (/ Mana MaxMana)))

(event EventOnStrengthChange
  (params (Strength :type Float%20%28single-precision%29) (MaxStrength :type Float%20%28single-precision%29))
  (bind _asbp_base_player_controller (Utilities|Casting|CastToBP_BasePlayerController (Pawn|GetController)))
  (Default|SetPercentage (Variables|/Game/UI/WBP_PrimaryUI.WBP_PrimaryUI_C|GetStrength_GlassBall (Variables|/Game/Blueprints/BP_BasePlayerController.BP_BasePlayerController_C|GetPrimaryUI _asbp_base_player_controller)) (/ Strength MaxStrength)))

(fn ConstructionScript
  (|CallParentFunction))