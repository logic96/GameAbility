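; BP_BaseCharacter is a Gameplay Ability System character base that grants initial abilities and triggers melee, dash and health regen.
; Sword and capsule overlaps with hostile characters send gameplay events for melee and dash damage, with an array filtering repeat capsule hits.
; It also handles knockback through a zero-friction impulse with optional hit stun, and death through a montage followed by delayed destruction.
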(event OnComponentBeginOverlap(SwordCollosion)
  (params (OverlappedComponent :type Primitive%20Component%20Object%20Reference) (OtherActor :type Actor%20Object%20Reference) (OtherComp :type Primitive%20Component%20Object%20Reference) (OtherBodyIndex :type Integer) (bFromSweep :type Boolean) (SweepResult :type Hit%20Result%20Structure%20%28by%20ref%29))
  ;[1 1 1] 武器碰撞
  (if (!= OtherActor self)
    (bind _asbp_base_character (Utilities|Casting|CastToBP_BaseCharacter OtherActor))
    (bind _returnvalue (Class|BaseCharacter|IsOtherHostile _asbp_base_character self))
    (if _returnvalue
      (Ability|SendGameplayEventtoActor self "(TagName=\"skill.melee.dealdamage\")" (Utilities|Struct|MakeGameplayEventData "" 0 _asbp_base_character)))))

(event OnComponentBeginOverlap(CapsuleComponent)
  (params (OverlappedComponent :type Primitive%20Component%20Object%20Reference) (OtherActor :type Actor%20Object%20Reference) (OtherComp :type Primitive%20Component%20Object%20Reference) (OtherBodyIndex :type Integer) (bFromSweep :type Boolean) (SweepResult :type Hit%20Result%20Structure%20%28by%20ref%29))
  (bind _self self)
  (bind _asbp_base_character (Utilities|Casting|CastToBP_BaseCharacter OtherActor))
  ;[1 1 1] 如果已经存在，则什么也不做
  (bind _alrealdyexist_ (CallFunction|CheckExistinArray _asbp_base_character))
  (if (not _alrealdyexist_)
    (bind _returnvalue (Class|BaseCharacter|IsOtherHostile _asbp_base_character _self))
    (if _returnvalue
      (Ability|SendGameplayEventtoActor self "(TagName=\"skill.dash.dealDamage\")" (Utilities|Struct|MakeGameplayEventData "" _self _asbp_base_character)))))

(event Custom|MeleeAttack
  (Abilities|TryActivateAbilitybyClass (Variables|Default|GetAbilitySystemComp) "/Game/Blueprints/Characters/Ability/Melee/GA_MeleeAttack.GA_MeleeAttack_C" true))

(event Custom|StartBlockSpeed)

(event Custom|EndBlockSpeed)

(event Custom|TryHealRegen
  (Abilities|TryActivateAbilitybyClass (Variables|Default|GetAbilitySystemComp) "/Game/Blueprints/Characters/Ability/HealthRegen/GA_HealthRegen.GA_HealthRegen_C" true))

(event Custom|TryDash
  (Abilities|TryActivateAbilitybyClass (Variables|Default|GetAbilitySystemComp) "/Game/Blueprints/Characters/Ability/Dash/GA_Dash.GA_Dash_C" true))

(event Custom|PushCharacter
  (params (Direction :type Vector) (Strength :type Float%20%28single-precision%29) (HitStunDuration :type Float%20%28single-precision%29))
  ;[1 1 1] 将位移看作是character自身的行为
  (Variables|Default|SetOriginalFriction (Variables|/Script/Engine.CharacterMovementComponent|GetGroundFriction (Variables|Character|GetCharacterMovement)))
  (Variables|/Script/Engine.CharacterMovementComponent|SetGroundFriction (Variables|Character|GetCharacterMovement) 0.0)
  (Physics|AddImpulse (Variables|Character|GetCharacterMovement) (* Direction Strength) true)
  ;[1 1 1] 添加击昏状态
  (if (> HitStunDuration 0.0)
    (Class|BaseCharacter|HitStun HitStunDuration))
  (Utilities|FlowControl|Delay 0.3)
  (Variables|/Script/Engine.CharacterMovementComponent|SetGroundFriction (Variables|Character|GetCharacterMovement) (Variables|Default|GetOriginalFriction)))

(event EventBeginPlay
  (Class|BaseCharacter|AquireAbilities (Variables|Default|GetInitialAbilities)))

(event Collision|EventActorBeginOverlap
  (params (OtherActor :type Actor%20Object%20Reference)))

(event EventDie
  ;[1 1 1] 播放死亡动画
  (Animation|Montage|PlayMontage (Variables|Character|GetMesh) "/Game/Blueprints/Characters/Animation/AM_ShibiDeath.AM_ShibiDeath" 0.9
    (:then
      (Utilities|FlowControl|Delay 2.0)
      (Actor|DestroyActor))))

(fn ConstructionScript)

(fn SetCollisiontoPawn
  (params (NewResponse :type ECollisionResponse%20Enum :default "ECR_Overlap"))
  (Collision|SetCollisionResponsetoChannel (Variables|Default|GetCapsuleComponent) "ECC_Pawn" NewResponse))

(fn CheckExistinArray
  (params (ColliderActor :type BP%20Base%20Character%20Object%20Reference%20%28by%20ref%29))
  (if (Utilities|Array|ContainsItem (Variables|Default|GetColliderActorArray) ColliderActor)
    (return true)
    (else
      (Utilities|Array|AddUnique (Variables|Default|GetColliderActorArray) ColliderActor)
      (return false))))