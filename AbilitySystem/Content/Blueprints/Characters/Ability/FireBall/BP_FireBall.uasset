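; BP_FireBall is the fireball ability actor that damages hostile characters it overlaps and destroys itself on a six-second timer.
; Its Sphere overlap casts both the other actor and its Instigator to BP_BaseCharacter and checks hostility between them.
; Hostile targets apply GE_FireballDamage to themselves through their own Ability System Component.
; An unconnected branch holds a spec-handle application and destroy-on-hit, so overlaps do not destroy the fireball.
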(event OnComponentBeginOverlap(Sphere)
  (params (OverlappedComponent :type Primitive%20Component%20Object%20Reference) (OtherActor :type Actor%20Object%20Reference) (OtherComp :type Primitive%20Component%20Object%20Reference) (OtherBodyIndex :type Integer) (bFromSweep :type Boolean) (SweepResult :type Hit%20Result%20Structure%20%28by%20ref%29))
  (bind _asbp_base_character (Utilities|Casting|CastToBP_BaseCharacter OtherActor))
  (bind _asbp_base_character_2 (Utilities|Casting|CastToBP_BaseCharacter (Game|GetInstigator)))
  (bind _returnvalue (Class|BaseCharacter|IsOtherHostile _asbp_base_character_2 _asbp_base_character))
  (if _returnvalue
    (GameplayEffects|ApplyGameplayEffectToSelf :self (Ability|GetAbilitySystemComponent _asbp_base_character) :GameplayEffectClass "/Game/Blueprints/Characters/Ability/FireBall/GE_FireballDamage.GE_FireballDamage_C")))

(event Custom|TimeToDie
  (Actor|DestroyActor))

(event EventBeginPlay
  (Utilities|Time|SetTimerbyEvent (delegate Custom|TimeToDie) 6.0))

(event Collision|EventActorBeginOverlap
  (params (OtherActor :type Actor%20Object%20Reference)))

(event EventTick
  (params (DeltaSeconds :type Float%20%28single-precision%29)))

(fn ConstructionScript)