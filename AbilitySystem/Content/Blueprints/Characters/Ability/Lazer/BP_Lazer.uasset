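; BP_Lazer is a laser beam ability actor that periodically reports hostile characters touched by its end point for damage.
; LazerEndDetector overlaps maintain a list of characters hostile to the instigator, which a looping timer sends to the instigator as a Skill.Lazer.DealDamage gameplay event with target data.
; Each tick, the detector's distance, which a collision-aware SpringArm shortens, offsets the beam's end bone through AnimBP_Lazer to fit its length.
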(event OnComponentBeginOverlap(LazerEndDetector)
  (params (OverlappedComponent :type Primitive%20Component%20Object%20Reference) (OtherActor :type Actor%20Object%20Reference) (OtherComp :type Primitive%20Component%20Object%20Reference) (OtherBodyIndex :type Integer) (bFromSweep :type Boolean) (SweepResult :type Hit%20Result%20Structure%20%28by%20ref%29))
  (bind _asbp_base_character (Utilities|Casting|CastToBP_BaseCharacter OtherActor))
  (bind _asbp_base_character_2 (Utilities|Casting|CastToBP_BaseCharacter (Game|GetInstigator)))
  (bind _returnvalue (Class|BaseCharacter|IsOtherHostile _asbp_base_character_2 _asbp_base_character))
  (if _returnvalue
    (Utilities|Array|AddUnique (Variables|Default|GetOverlapingActors) _asbp_base_character)))

(event OnComponentEndOverlap(LazerEndDetector)
  (params (OverlappedComponent :type Primitive%20Component%20Object%20Reference) (OtherActor :type Actor%20Object%20Reference) (OtherComp :type Primitive%20Component%20Object%20Reference) (OtherBodyIndex :type Integer))
  (bind _asbp_base_character (Utilities|Casting|CastToBP_BaseCharacter OtherActor))
  (Utilities|Array|RemoveItem (Variables|Default|GetOverlapingActors) _asbp_base_character))

(event Custom|SendDealDamageEvent
  ;[1 1 1] 每三秒发送一次,需要Looping
  (if (Math|Conversions|ToBoolean(Integer) (Utilities|Array|Length (Variables|Default|GetOverlapingActors))) ; 这里不用检查是否为0，在WaitEvent里要保证调用Cost的检查
    _
    (else
      _))
  (Ability|SendGameplayEventtoActor (Game|GetInstigator) "(TagName=\"Skill.Lazer.DealDamage\")" (Utilities|Struct|MakeGameplayEventData "" 0 0 0 0 "()" "(GameplayTags=)" "(GameplayTags=)" 0.0 (Ability|TargetData|AbilityTargetDatafromActorArray (Variables|Default|GetOverlapingActors)))))

(event EventBeginPlay
  (Variables|Default|SetBeamOriginalLength (Math|Vector|VectorLength (- (Transformation|GetSocketLocation (Variables|Default|GetLazerMesh) "end") (Transformation|GetActorLocation))))
  ;[1 1 1] 每三秒发送一次,需要Looping
  (Utilities|Time|SetTimerbyEvent (delegate Custom|SendDealDamageEvent) 0.3 true))

(event Collision|EventActorBeginOverlap
  (params (OtherActor :type Actor%20Object%20Reference)))

(event EventTick
  (params (DeltaSeconds :type Float%20%28single-precision%29))
  (bind _asanim_bp_lazer (Utilities|Casting|CastToAnimBP_Lazer (Components|SkeletalMesh|GetAnimInstance (Variables|Default|GetLazerMesh))))
  (Variables|/Game/Blueprints/Characters/Ability/Lazer/LazerAsset/AnimBP_Lazer.AnimBP_Lazer_C|SetEndBoneOffset _asanim_bp_lazer (Math|Vector|MakeVector (- (Math|Vector|VectorLength (- (Transformation|GetWorldLocation (Variables|Default|GetLazerEndDetector)) (Transformation|GetActorLocation))) (Variables|Default|GetBeamOriginalLength)) 0.0 0.0)))

(fn ConstructionScript)