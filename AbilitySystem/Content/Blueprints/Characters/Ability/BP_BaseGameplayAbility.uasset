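; Base gameplay ability Blueprint that provides a helper for showing its cooldown on the player's ability UI.
; DoUICoolDown gets player controller 0 as BP_BasePlayerController and scans the slots in its PrimaryUI.
; Every slot whose ability class matches this ability's GetAbilityInfo result starts its cooldown display.
; The activate and end events are unimplemented placeholders, and nothing in this graph calls the helper.
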(event Ability|EventActivateAbility)

(event Ability|EventOnEndAbility
  (params (bWasCancelled :type Boolean)))

(fn DoUICoolDown
  ;[1 1 1] 当前技能发动时，找到对应图标，调用startCoolDown
  (bind _asbp_base_player_controller (Utilities|Casting|CastToBP_BasePlayerController (Game|GetPlayerController 0)))
  (for _array_element (Variables|/Game/UI/WBP_PrimaryUI.WBP_PrimaryUI_C|GetSlots (Variables|/Game/Blueprints/BP_BasePlayerController.BP_BasePlayerController_C|GetPrimaryUI _asbp_base_player_controller))
    (bind _returnvalue (Class|BaseGameplayAbility|GetAbilityInfo))
    (if (== (.AbilityClass (Utilities|Struct|BreakGameplayAbilityInfo _returnvalue)) (.abilityclass (Variables|/Game/UI/WBP_Ability_Slot.WBP_Ability_Slot_C|GetAbilityInfo _array_element)))
      (Default|StartCoolDown _array_element))))